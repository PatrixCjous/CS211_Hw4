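; BP_SeaWater is a sea water actor that bounces physics objects upward when they enter it.
; When a simulating component begins overlapping the Volume, it keeps its horizontal velocity, drops its vertical velocity and receives a fixed, mass-independent upward impulse.
; The construction script creates a dynamic M_SeaWater material on the WaterLevel component and feeds it the Tiling and Timing variables.
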(event OnComponentBeginOverlap(Volume)
  (params (OtherActor :type Actor%20Object%20Reference) (OtherComp :type Primitive%20Component%20Object%20Reference) (OtherBodyIndex :type Integer) (bFromSweep :type Boolean) (SweepResult :type Hit%20Result%20Structure%20%28by%20ref%29))
  (if (Physics|IsSimulatingPhysics OtherComp "None")
    (bind _returnvalue (Physics|GetPhysicsLinearVelocity OtherComp "None"))
    (Physics|SetPhysicsLinearVelocity OtherComp (Math|Vector|MakeVector (.x _returnvalue) (.y _returnvalue) 0.0) false "None")
    (Physics|AddImpulse OtherComp "0, 0,300.000000" "None" true)))

(fn ConstructionScript
  (bind _returnvalue (Rendering|Material|CreateDynamicMaterialInstance (Variables|Default|GetWaterLevel) 0 "/Game/Materials/M_SeaWater.M_SeaWater" :!class /Script/Engine.PrimitiveComponent))
  (bind _output_get (Variables|Default|SetwaterMat _returnvalue))
  (Rendering|Material|SetScalarParameterValue _output_get "Tiling" (Variables|Default|GetTiling) :!class /Script/Engine.MaterialInstanceDynamic)
  (Rendering|Material|SetScalarParameterValue _output_get "Timing" (Variables|Default|GetTiming) :!class /Script/Engine.MaterialInstanceDynamic))