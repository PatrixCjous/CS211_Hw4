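; Stereo speaker pair actor that plays the audio of the movie assigned to its MoviePlayer reference.
; The construction script places the right and left speakers symmetrically along X using Separation.
; PlayMovie loads the sound into both audio components and starts at zero, or resumes from AudioTime after PauseMovie.
; Tick advances AudioTime whenever NoSound is false, even while paused; StopMovie sets NoSound so playback restarts.
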(event EventTick
  (params (DeltaSeconds :type Float%20%28single-precision%29))
  (if (not (Variables|Default|GetnoSound))
    (Variables|Default|SetaudioTime (+ DeltaSeconds (Variables|Default|GetaudioTime)))))

(fn ConstructionScript
  (bind _separation (Variables|Default|Getseparation))
  (Transformation|SetRelativeLocation (Variables|Default|GetBocinaR) (Math|Vector|MakeVector _separation 0.0 0.0) false)
  (Transformation|SetRelativeLocation (Variables|Default|GetBocinaL) (Math|Vector|MakeVector (* _separation -1.0) 0.0 0.0) false))

(fn PlayMovie
  (bind _movieplayer (Variables|Default|GetmoviePlayer))
  (bind _audior (Variables|Default|GetAudioR))
  (bind _audiol (Variables|Default|GetAudioL))
  (bind _movie (Variables|/Game/Blueprints/Homework/BP_MoviePlayer.BP_MoviePlayer_C|Getmovie _movieplayer))
  (bind _audio (Variables|/Game/Blueprints/Homework/BP_Movie.BP_Movie_C|Getaudio _movie))
  (if (Variables|Default|GetnoSound)
    (Utilities|IsValid _movie
      (:Is%20Valid
        (Utilities|FlowControl|Sequence
          (:then_0
            (Audio|Components|Audio|SetSound _audior _audio))
          (:then_1
            (Audio|Components|Audio|SetSound _audiol _audio))
          (:then_2
            (Audio|Components|Audio|Play _audior 0.0))
          (:then_3
            (Audio|Components|Audio|Play _audiol 0.0))
          (:then_4
            (Variables|Default|SetnoSound false)
            (Variables|Default|SetaudioTime 0.0)))))
    (else
      (Utilities|FlowControl|Sequence
        (:then_0
          (Audio|Components|Audio|Play (Variables|Default|GetAudioL) (Variables|Default|GetaudioTime)))
        (:then_1
          (Audio|Components|Audio|Play (Variables|Default|GetAudioR) (Variables|Default|GetaudioTime)))))))

(fn StopMovie
  (CallFunction|PauseMovie)
  (Variables|Default|SetnoSound true))

(fn PauseMovie
  (if (not (Variables|Default|GetnoSound))
    (Utilities|FlowControl|Sequence
      (:then_0
        (Audio|Components|Audio|Stop (Variables|Default|GetAudioR)))
      (:then_1
        (Audio|Components|Audio|Stop (Variables|Default|GetAudioL))))))