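; BP_MoviePlayer is a movie player device that accepts a BP_Movie object dropped into its trigger box.
; When empty, it stores the first overlapping movie, zeroes its velocity and snaps it above the player's origin, then Tick spins it around yaw.
; When that movie leaves the box, it clears the reference and stops MovieScreen and Speakers.
; Playback start is not handled in this Blueprint.
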(event OnComponentBeginOverlap(Box)
  (params (OtherActor :type Actor%20Object%20Reference) (OtherComp :type Primitive%20Component%20Object%20Reference) (OtherBodyIndex :type Integer) (bFromSweep :type Boolean) (SweepResult :type Hit%20Result%20Structure%20%28by%20ref%29))
  (bind _asbp_movie (Utilities|Casting|CastToBP_Movie OtherActor))
  (Utilities|IsValid (Variables|Default|Getmovie)
    (:Is%20Not%20Valid
      (bind _output_get (Variables|Default|Setmovie _asbp_movie))
      (Physics|SetPhysicsLinearVelocity _output_get "0, 0, 0" false "None")
      (Transformation|SetWorldLocation _output_get (+ (Transformation|GetActorLocation) "0, 0,100.000000") false))))

(event OnComponentEndOverlap(Box)
  (params (OtherActor :type Actor%20Object%20Reference) (OtherComp :type Primitive%20Component%20Object%20Reference) (OtherBodyIndex :type Integer))
  (if (== OtherActor (Variables|Default|Getmovie))
    (Variables|Default|Setmovie 0)
    (Default|StopMovie (Variables|Default|GetmovieScreen))
    (Default|StopMovie (Variables|Default|Getspeakers))))

(event EventTick
  (params (DeltaSeconds :type Float%20%28single-precision%29))
  (bind _movie (Variables|Default|Getmovie))
  (Utilities|IsValid _movie
    (:Is%20Valid
      (Transformation|SetWorldRotation _movie (Math|Rotator|MakeRotator 0.0 (+ (.yaw (Transformation|GetWorldRotation _movie)) (* 1e+02 (Utilities|Time|GetWorldDeltaSeconds))) 0.0) false))))

(fn ConstructionScript)