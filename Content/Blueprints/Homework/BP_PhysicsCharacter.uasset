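; Physics-driven player character that moves by setting the linear velocity of its static mesh.
; Each tick, forward, right and up input is rotated by the camera's yaw, scaled by moving speed and delta time, and added to the current velocity.
; The TurnRate axis adds controller yaw, scaled by turn rate and delta time.
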(event EventTick
  (params (DeltaSeconds :type Float%20%28single-precision%29))
  (Physics|SetPhysicsLinearVelocity (Variables|Default|GetStaticMesh) (+ (Transformation|GetVelocity) (* (* (Math|Vector|RotateVector (Math|Vector|MakeVector (Input|AxisValues|GetMoveForward) (Input|AxisValues|GetMoveRight) (Input|AxisValues|GetMoveUp)) (Math|Rotator|MakeRotator 0.0 (.yaw (Transformation|GetWorldRotation (Variables|Default|GetCamera))) 0.0)) (Variables|Default|GetMovingSpeed)) (Utilities|Time|GetWorldDeltaSeconds))) false "None"))

(event Input|AxisEvents|InputAxisTurnRate
  (params (AxisValue :type Float%20%28single-precision%29))
  (Pawn|Input|AddControllerYawInput (* AxisValue (Utilities|Time|GetWorldDeltaSeconds) (Variables|Default|GetTurnRateScalar))))

(fn ConstructionScript)