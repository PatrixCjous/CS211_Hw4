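; BP_Screen is a movie screen actor that plays, pauses and stops video on its Screen component.
; PlayMovie resumes the cached media player, or applies the material from MoviePlayer's current Movie to the screen, then caches and plays that movie's media player.
; PauseMovie pauses only during playback, while StopMovie rewinds, pauses and clears the cached player so the next play reloads from MoviePlayer.
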(event EventBeginPlay)

(event EventActorBeginOverlap
  (params (OtherActor :type Actor%20Object%20Reference)))

(event EventTick
  (params (DeltaSeconds :type Float%20%28single-precision%29)))

(fn ConstructionScript)

(fn PlayMovie
  (bind _movieplayer (Variables|Default|GetmoviePlayer))
  (bind _movie (Variables|/Game/Blueprints/Homework/BP_MoviePlayer.BP_MoviePlayer_C|Getmovie _movieplayer))
  (Utilities|IsValid (Variables|Default|GetcurrentMediaPlayer)
    (:Is%20Valid
      (Media|MediaPlayer|Play (Variables|Default|GetcurrentMediaPlayer) :!class /Script/MediaAssets.MediaPlayer))
    (:Is%20Not%20Valid
      (Utilities|IsValid _movie
        (:Is%20Valid
          (Rendering|Material|SetMaterial (Variables|Default|GetScreen) 0 (Variables|/Game/Blueprints/Homework/BP_Movie.BP_Movie_C|Getmovie _movie))
          (bind _output_get (Variables|Default|SetcurrentMediaPlayer (Variables|/Game/Blueprints/Homework/BP_Movie.BP_Movie_C|GetmediaPlayer _movie)))
          (Media|MediaPlayer|Play _output_get :!class /Script/MediaAssets.MediaPlayer))))))

(fn PauseMovie
  (bind _currentmediaplayer (Variables|Default|GetcurrentMediaPlayer))
  (Utilities|IsValid _currentmediaplayer
    (:Is%20Valid
      (if (Audio|Components|Audio|IsPlaying _currentmediaplayer)
        (Sequencer|Player|Pause _currentmediaplayer)))))

(fn StopMovie
  (Utilities|IsValid (Variables|Default|GetcurrentMediaPlayer)
    (:Is%20Valid
      (Class|MediaPlayer|Rewind (Variables|Default|GetcurrentMediaPlayer))
      (Sequencer|Player|Pause (Variables|Default|GetcurrentMediaPlayer))
      (Variables|Default|SetcurrentMediaPlayer 0))))