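; BP_Curtain is a curtain that gets pushed by physics when its Use event fires.
; Use applies an impulse to each of the four Hanger components in sequence, along the forward vector of the first player's pawn.
; The impulse is applied as a velocity change, so the hangers' mass does not affect the push.
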(event EventUse
  (bind _returnvalue (Game|Player|GetPlayerPawn 0))
  (bind _returnvalue_2 (Transformation|GetActorForwardVector _returnvalue))
  (bind _returnvalue_3 (* _returnvalue_2 7e+02))
  (Utilities|FlowControl|Sequence
    (:then_0
      (Physics|AddImpulse (Variables|Default|GetHanger1) _returnvalue_3 "None" true))
    (:then_1
      (Physics|AddImpulse (Variables|Default|GetHanger2) _returnvalue_3 "None" true))
    (:then_2
      (Physics|AddImpulse (Variables|Default|GetHanger3) _returnvalue_3 "None" true))
    (:then_3
      (Physics|AddImpulse (Variables|Default|GetHanger4) _returnvalue_3 "None" true))))

(fn ConstructionScript)